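; Game mode for a runner game that builds the initial track of floor tiles when play begins.
; BeginPlay calls AddFloor once per NumberOfTiles, spawning a BP_Floor and storing it in the FloorTiles array.
; Each new tile's attach point becomes the next SpawnTransform, so the tiles chain end to end.
; ExtendFloor is an empty stub, and Tick does nothing.
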(event EventBeginPlay
  (for _index (range 0 (- (Variables|Default|GetNumberOfTiles) 1))
    (CallFunction|AddFloor)))

(event EventTick
  (params (DeltaSeconds :type Float%20%28single-precision%29)))

(fn ConstructionScript)

(fn AddFloor
  (bind _returnvalue (Game|SpawnActorfromClass "/Game/Runner/Blueprints/BP_Floor.BP_Floor_C" (Variables|Default|GetSpawnTransform) "Undefined" "MultiplyWithRoot" 0 0))
  (bind _returnvalue_2 (Default|GetAttachPoint _returnvalue))
  (Variables|Default|SetSpawnTransform _returnvalue_2)
  (Utilities|Array|Add (Variables|Default|GetFloorTiles) _returnvalue))

(fn ExtendFloor)